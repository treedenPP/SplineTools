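; Click-to-move controller that sends the level's MyAICharacter to the point under the mouse and visualizes its path.
; BeginPlay caches the character, and each left click runs a Visibility trace from the camera through the cursor to set the destination for AI MoveTo.
; As the move is issued, a separate synchronous navigation query supplies path points, drawn as debug lines and spheres with their count printed.
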(event EventBeginPlay
  (bind _returnvalue (Actor|GetActorOfClass "/Script/SplineTools.MyAICharacter"))
  (Utilities|IsValid _returnvalue
    (:Is%20Valid
      (Variables|Default|SetAI _returnvalue))))

(event EventTick
  (params (DeltaSeconds :type Float%20%28single-precision%29)))

(event Input|MouseEvents|LeftMouseButton
  (params (Key :type Key%20Structure :default "None"))
  (:Pressed
    (Utilities|Trace)
    (AI|AIMoveTo (Variables|Default|GetAI) (Variables|Default|GetEndLocation) 0 5.0 false
      (:then
        (bind _returnvalue (Class|NavigationSystemV1|FindPathtoLocationSynchronously (Transformation|GetActorLocation (Variables|Default|GetAI)) (Variables|Default|GetEndLocation) 0 0))
        (for (_array_element _array_index) (Variables|/Script/NavigationSystem.NavigationPath|GetPathPoints _returnvalue)
          (if (!= _array_index (- (Utilities|Array|Length (Variables|/Script/NavigationSystem.NavigationPath|GetPathPoints _returnvalue)) 1))
            (Rendering|Debug|DrawDebugLine :LineStart _array_element :LineEnd (Utilities|Array|Get(acopy) (Variables|/Script/NavigationSystem.NavigationPath|GetPathPoints _returnvalue) (+ _array_index 1)) :Duration 2.0 :Thickness 2.0))
          (Rendering|Debug|DrawDebugSphere _array_element 2e+01 12 "(R=1.000000,G=0.000000,B=0.000000,A=1.000000)" 2.0 2.0))
        (Development|PrintString (Utilities|String|Append "Point Number" (Utilities|String|ToString(Integer) (Utilities|Array|Length (Variables|/Script/NavigationSystem.NavigationPath|GetPathPoints _returnvalue)))))))))

(fn ConstructionScript)